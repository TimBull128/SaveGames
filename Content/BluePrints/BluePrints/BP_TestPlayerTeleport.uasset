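; Test portal actor that teleports the player to a linked EndPortal while keeping momentum, with cinematic follow cameras.
; BeginPlay feeds the EndPortal's capture camera into a viewport-sized render target on the plane's material; Tick passes it the player camera transform within an angle range.
; A front trigger precomputes position, control rotation and velocity for the teleport box to apply.
; Afterwards, two follow cameras are meant to animate the transition before returning to the player view.
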(event `self.ReceiveBeginPlay`
  (bind (_returnvalue_x _returnvalue_y) (`KismetMathLibrary.BreakVector2D` (`WidgetLayoutLibrary.GetViewportSize`)))
  (`|ExecutionSequence`
    (:`then_0`
      ; Get Player Information
      (bind _player (`/Game/BluePrints/Classes/BPF_Casts.Get Player Character` 0))
      (set `self.Player` _player)
      (bind _returnvalue (`/Game/BluePrints/Classes/BPF_Casts.Get Player Controller` 0))
      (set `self.Player Controller` _returnvalue)
      (bind _returnvalue_2 (`/Game/BluePrints/Classes/BPF_Casts.Get Player Camera Manager` 0))
      (set `self.Player Camera Manager` _returnvalue_2)
      (bind _outactors (`GameplayStatics.GetAllActorsOfClass` "/Game/BluePrints/BluePrints/BP_Portal_Camera.BP_Portal_Camera_C"))
      (set `self.Portal Followup Cameras` _outactors)
      (bind _player_pawn (`/Game/BluePrints/Classes/BPF_Casts.Get Player Pawn` 0))
      (set `self.Player Pawn` _player_pawn))
    (:`then_1`
      (`self.SetTickGroup` "TG_PostUpdateWork")
      ;;[0.04459 0.15 0.03479 0.5] Portal Material
      ;;;[0.1082 0.15 0.1159 0.5] Create Material Instance
      (bind _returnvalue_3 (`KismetMaterialLibrary.CreateDynamicMaterialInstance` "/Game/BluePrints/Materials/M_Portal.M_Portal"))
      (bind _output_get (set `self.Portal Material` _returnvalue_3))
      (`PrimitiveComponent.SetMaterial` (`self.Portal Plane`) 0 _output_get)
      ;;;[0.1266 0.15 0.1338 0.5] Create Render Target
      (bind _returnvalue_4 (`KismetRenderingLibrary.CreateRenderTarget2D` (`KismetMathLibrary.FTrunc` _returnvalue_x) (`KismetMathLibrary.FTrunc` _returnvalue_y)))
      (bind _output_get_2 (set `self.Portal Render Target` _returnvalue_4))
      ;;;[0.1251 0.15 0.1229 0.5] Setting Textures to Plane
      (bind _portal_material (`self.Portal Material`)
        (:`then`
          (`MaterialInstanceDynamic.SetTextureParameterValue` _portal_material "Texture" _output_get_2)
          (bind _end_portal (`self.End Portal`)
            (:`then`
              (set `SceneCaptureComponent2D.TextureTarget` (`self.Portal Render Target`) (`/Game/BluePrints/BluePrints/BP_TestPlayer_Teleport_End.Portal_cam` _end_portal)))
            (:`else`)))
        (:`else`)))))

(event `self.ReceiveTick`
  (params (DeltaSeconds :type "Float (single-precision)"))
  (bind (_camera_pos_location _camera_pos_rotation) (`KismetMathLibrary.BreakTransform` (`self.Camera Pos`)))
  (bind _output (`|GetArrayItem` (`self.Portal Followup Cameras`)))
  (bind _returnvalue (`SceneComponent.K2_GetComponentToWorld` (`/Game/BluePrints/BluePrints/BP_TestPlayer_Teleport_End.Portal_cam` (`self.End Portal`))))
  (bind _returnvalue_2 (`KismetMathLibrary.FindLookAtRotation` (`SceneComponent.K2_GetComponentLocation` (`self.Portal Plane`)) (`SceneComponent.K2_GetComponentLocation` (`Actor.RootComponent` (`self.Player Camera Manager`)))))
  (bind _yaw (.yaw _returnvalue_2))
  (`|ExecutionSequence`
    (:`then_0`
      ;[0.01378 0.15 0.007548 0.5] Updating the Portal Camera Rotation
      ;; Get the Look At position for the portal camera
      (if (>= _yaw 0.0)
        (set `self.Portal Camera Rotation` _returnvalue_2)
        (else
          (bind _output_get (set `self.Portal Camera Rotation` (`KismetMathLibrary.MakeRotator` (.roll _returnvalue_2) (.pitch _returnvalue_2) (+ _yaw 360.0))))))
      (bind _yaw_2 (.yaw _output_get))
      ; Get Player Information
      ;;; Check if the angle is within bounds of the camera
      (if (and (> _yaw_2 90.0) (< _yaw_2 270.0))
        (set `/Game/BluePrints/BluePrints/BP_TestPlayer_Teleport_End.Portal Cam Rotation` (`SceneComponent.K2_GetComponentToWorld` (`PlayerCameraManager.TransformComponent` (`self.Player Camera Manager`))) (`self.End Portal`))))
    (:`then_1`
      ;[0.02982 0.04769 0.15 0.5] Followup cameras
      (`self.follow cam active`
        (:`then`
          ;; Set Transform of the pre teleport camera
          (`SceneComponent.K2_SetWorldLocationAndRotation` (`self.Last Known PlayerCam Pos`) _camera_pos_location _camera_pos_rotation false false)
          (`SceneComponent.K2_SetWorldLocationAndRotation` (`Actor.RootComponent` (`|GetArrayItem` (`self.Portal Followup Cameras`))) _camera_pos_location _camera_pos_rotation false false)
          ;; Set Transform of Post Teleport Followup Camera
          (`SceneComponent.K2_SetWorldTransform` (`/Game/BluePrints/BluePrints/BP_Portal_Camera.DefaultSceneRoot` (`|GetArrayItem` (`self.Portal Followup Cameras`) 1)) (`KismetMathLibrary.MakeTransform` (.location _returnvalue) (`KismetMathLibrary.MakeRotator` (.roll (.rotation _returnvalue)))) false false)
          ;; change camera to the first portal cam and animate
          (bind _returnvalue_3 (`self.Animate Followup Cam` _output (`/Game/BluePrints/BluePrints/BP_Portal_Camera.DefaultSceneRoot` _output) (`SceneComponent.K2_GetComponentToWorld` (`self.end followup cam pos`)) 1.0 10.0))
          ;; Change camera to the second portal cam
          (if _returnvalue_3
            (`KismetSystemLibrary.Delay` 1.0)
            (`/Game/BluePrints/Classes/BPF_Casts.Camera Change` (`self.Player Controller`) (`|GetArrayItem` (`self.Portal Followup Cameras`) 1))
            ;; reset the camera to player cam
            (`/Game/BluePrints/Classes/BPF_Casts.Camera Change` (`self.Player Controller`) (`self.Player`) 5.0)
            (set `self.follow cam active` false)
            (set `self.Should Teleport` false)
            (set `/Game/BluePrints/BluePrints/BP_TestPlayer_Teleport_End.Should Rotate` true (`self.End Portal`))))
        (:`else`)))))

(event `self.Teleport Box.OnComponentBeginOverlap`
  (params (OverlappedComponent :type "PrimitiveComponent Object Reference") (OtherActor :type "Actor Object Reference") (OtherComp :type "PrimitiveComponent Object Reference") (OtherBodyIndex :type Integer) (bFromSweep :type Boolean) (SweepResult :type "HitResult Structure (by ref)"))
  (bind (_player_pos_location _player_pos_rotation) (`KismetMathLibrary.BreakTransform` (`self.Player Pos`)))
  ;[0.03185 0.04853 0.15 0.5] Teleport
  ;; Check if player is in front of the portal when box hit
  (if (and (== OtherActor "/Game/ThirdPerson/Blueprints/BP_ThirdPersonCharacter.BP_ThirdPersonCharacter") (`self.Should Teleport`))
    ;; Set Player Position
    (`SceneComponent.K2_SetWorldLocationAndRotation` (`self.New Player Pos`) _player_pos_location _player_pos_rotation false false)
    (`SceneComponent.K2_SetWorldLocationAndRotation` (`Actor.RootComponent` (`self.Player`)) _player_pos_location _player_pos_rotation false false)
    ;; Set Control Rotation
    (`Controller.SetControlRotation` (`self.Player Controller`) (`self.Control Rotation`))
    ;; Keep momentum
    (`Character.LaunchCharacter` (`self.Player`) (`self.Velocity`) true true)
    ;; Teleport
    (set `self.follow cam active` true)
    (set `/Game/BluePrints/BluePrints/BP_TestPlayer_Teleport_End.Should Rotate` false (`self.End Portal`))))

(event `self.Actor in front.OnComponentBeginOverlap`
  (params (OverlappedComponent :type "PrimitiveComponent Object Reference") (OtherActor :type "Actor Object Reference") (OtherComp :type "PrimitiveComponent Object Reference") (OtherBodyIndex :type Integer) (bFromSweep :type Boolean) (SweepResult :type "HitResult Structure (by ref)"))
  (bind (_returnvalue_location _returnvalue_rotation _returnvalue_scale) (`KismetMathLibrary.BreakTransform` (`SceneComponent.K2_GetComponentToWorld` (`Actor.RootComponent` (`self.Player`)))))
  (bind (_returnvalue_location_2 _returnvalue_rotation_2) (`KismetMathLibrary.BreakTransform` (`SceneComponent.K2_GetComponentToWorld` (`/Game/BluePrints/BluePrints/BP_TestPlayer_Teleport_End.Frame` (`self.End Portal`)))))
  (if (== OtherActor null)
    ; Get player details
    ;; get control rotation
    (set `self.Control Rotation` (`/Game/BluePrints/BluePrints/BPF_Translation.Update Rotator` (`KismetMathLibrary.MakeRotFromX` (`self.GetActorForwardVector` (`self.Player Controller`))) _returnvalue_rotation_2))
    ;; Get new Position of the player
    (set `self.Player Pos` (`KismetMathLibrary.MakeTransform` (+ _returnvalue_location_2 (`KismetMathLibrary.InverseTransformLocation` (`SceneComponent.K2_GetComponentToWorld` (`self.Portal Plane`)) _returnvalue_location)) (`/Game/BluePrints/BluePrints/BPF_Translation.Update Rotator` _returnvalue_rotation_2 _returnvalue_rotation) _returnvalue_scale))
    ;; Set the velocity of the player
    (set `self.Velocity` (`KismetMathLibrary.GreaterGreater_VectorRotator` (`MovementComponent.Velocity` (`Pawn.GetMovementComponent` (`self.Player Pawn`))) (`SceneComponent.K2_GetComponentRotation` (`/Game/BluePrints/BluePrints/BP_TestPlayer_Teleport_End.Portal_cam` (`self.End Portal`)))))
    (set `self.Should Teleport` true)))

(fn `Animate Followup Cam`
  (params (`Target Camera` :type "Actor Object Reference") (`Camera Base` :type "SceneComponent Object Reference") (`Final  World Transform` :type "Transform Structure") (InterpSpeed :type "Float (single-precision)") (ErrorTolerance :type "Float (single-precision)"))
  (returns (ReturnValue :type Boolean))
  (bind _location (.location `Final  World Transform`))
  (bind _returnvalue (`GameplayStatics.GetWorldDeltaSeconds`))
  (bind (_returnvalue_location _returnvalue_rotation) (`KismetMathLibrary.BreakTransform` (`SceneComponent.K2_GetComponentToWorld` `Camera Base`)))
  (`/Game/BluePrints/Classes/BPF_Casts.Camera Change` (`self.Player Controller`) `Target Camera`)
  (`SceneComponent.K2_SetWorldLocationAndRotation` `Camera Base` (`KismetMathLibrary.VInterpTo` _returnvalue_location _location _returnvalue InterpSpeed) (`KismetMathLibrary.RInterpTo` _returnvalue_rotation (.rotation `Final  World Transform`) _returnvalue InterpSpeed) false false)
  (return (== _location (`SceneComponent.K2_GetComponentLocation` `Camera Base`) :`ErrorTolerance` ErrorTolerance)))

(fn `UserConstructionScript`)