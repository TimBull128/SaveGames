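; BP_TestGimbol is a test Blueprint comparing plain local rotation with a per-axis gimbal setup.
; Three input actions each apply a fixed local-rotation step on one axis to both the Standard component and the matching X, Y or Z component.
; ResetGimbolAxis then caches the Cube's world rotation, zeroes that axis component's relative rotation and restores the Cube's rotation, so the axis components never accumulate rotation.
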(event `EnhancedInput|/Game/Input/Actions/IA_RotateX`
  (params (ActionValue :type Boolean) (ElapsedSeconds :type "Float (double-precision)") (TriggeredSeconds :type "Float (double-precision)") (InputAction :type "InputAction Object Reference" :default "/Game/Input/Actions/IA_RotateX.IA_RotateX"))
  (:`Triggered`
    (`|ExecutionSequence`
      (:`then_0`
        (`SceneComponent.K2_AddLocalRotation` (`self.Standard`) (`KismetMathLibrary.MakeRotator` 5.0) false false))
      (:`then_1`
        (`SceneComponent.K2_AddLocalRotation` (`self.X`) (`KismetMathLibrary.MakeRotator` 5.0) false false)
        (`self.Reset Gimbol Axis` (`self.X`))))))

(event `EnhancedInput|/Game/Input/Actions/IA_RotateY`
  (params (ActionValue :type Boolean) (ElapsedSeconds :type "Float (double-precision)") (TriggeredSeconds :type "Float (double-precision)") (InputAction :type "InputAction Object Reference" :default "/Game/Input/Actions/IA_RotateY.IA_RotateY"))
  (:`Triggered`
    (`|ExecutionSequence`
      (:`then_0`
        (`SceneComponent.K2_AddLocalRotation` (`self.Standard`) (`KismetMathLibrary.MakeRotator` 0.0 5.0) false false))
      (:`then_1`
        (`SceneComponent.K2_AddLocalRotation` (`self.Y`) (`KismetMathLibrary.MakeRotator` 0.0 5.0) false false)
        (`self.Reset Gimbol Axis` (`self.Y`))))))

(event `EnhancedInput|/Game/Input/Actions/IA_RotateZ`
  (params (ActionValue :type Boolean) (ElapsedSeconds :type "Float (double-precision)") (TriggeredSeconds :type "Float (double-precision)") (InputAction :type "InputAction Object Reference" :default "/Game/Input/Actions/IA_RotateZ.IA_RotateZ"))
  (:`Triggered`
    (`|ExecutionSequence`
      (:`then_0`
        (`SceneComponent.K2_AddLocalRotation` (`self.Standard`) (`KismetMathLibrary.MakeRotator` 0.0 0.0 5.0) false false))
      (:`then_1`
        (`SceneComponent.K2_AddLocalRotation` (`self.Z`) (`KismetMathLibrary.MakeRotator` 0.0 0.0 5.0) false false)
        (`self.Reset Gimbol Axis` (`self.Z`))))))

(fn `Reset Gimbol Axis`
  (params (`Gimbol Direction` :type "SceneComponent Object Reference"))
  (set `self.CurrentRotation` (`SceneComponent.K2_GetComponentRotation` (`self.Cube`)))
  (`SceneComponent.K2_SetRelativeRotation` :`self` `Gimbol Direction`)
  (`SceneComponent.K2_SetWorldRotation` (`self.Cube`) (`self.CurrentRotation`) false false))

(fn `UserConstructionScript`)