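; Base interactable Blueprint that supplies a name, description and configurable outline highlight for targeted objects.
; On BeginPlay it creates a dynamic instance of the outline material, falling back to MI_Testoutline when none is set.
; SetOutlineMaterial pushes the stored colour and width into that instance and applies it as the given mesh's overlay material when targeted, otherwise clearing the overlay.
; Setters and getters expose the outline settings.
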(event `self.ReceiveBeginPlay`
  (`self.Make Outline Material`))

(event `/Game/BluePrints/Classes/BPI_Interact.Make Outline Material`
  ;[0.01602 0.15 0.004196 0.5] Creation of the Dynamic Material Instance.
  (bind _outline_material (`self.Outline Material`)
    (:`then`
      (bind _returnvalue (`KismetMaterialLibrary.CreateDynamicMaterialInstance` _outline_material))
      (set `self.Dynamic Outline Material` _returnvalue))
    (:`else`
      (bind _output_get (set `self.Outline Material` "/Game/BluePrints/Materials/MI_Testoutline.MI_Testoutline"))
      (bind _returnvalue_2 (`KismetMaterialLibrary.CreateDynamicMaterialInstance` _output_get))
      (set `self.Dynamic Outline Material` _returnvalue_2))))

(event `/Game/BluePrints/Classes/BPI_Interact.Update Outline Colour`
  ;[0.01602 0.15 0.004196 0.5] Setting Outline Colour
  (`MaterialInstanceDynamic.SetVectorParameterValue` (`self.Dynamic Outline Material`) "Emissive Colour" (`self.Outline Colour`)))

(event `/Game/BluePrints/Classes/BPI_Interact.Update Outline Width`
  ;[0.01602 0.15 0.004196 0.5] Setting outline Width
  (`MaterialInstanceDynamic.SetScalarParameterValue` (`self.Dynamic Outline Material`) "Line width" (`self.Outline Width`)))

(event `/Game/BluePrints/Classes/BPI_Interact.Set Outline Material`
  (params (`Target Mesh` :type "MeshComponent Object Reference"))
  ;[0.01602 0.15 0.004196 0.5] Set the Material on or off
  (`self.Is Targeted?`
    (:`then`
      (`self.Update Outline Colour`)
      (`/Game/BluePrints/Classes/BPI_Interact.Update Outline Width`)
      (`MeshComponent.SetOverlayMaterial` `Target Mesh` (`self.Dynamic Outline Material`)))
    (:`else`
      (`MeshComponent.SetOverlayMaterial` `Target Mesh` null))))

(event `/Game/BluePrints/Classes/BPI_Interact.Set Outline Colour`
  (params (`Outline Colour` :type "LinearColor Structure"))
  (set `self.Outline Colour` `Outline Colour`))

(event `/Game/BluePrints/Classes/BPI_Interact.Set Outline Width`
  (params (`Outline Width` :type "Float (double-precision)"))
  (set `self.Outline Width` `Outline Width`))

(event `/Game/BluePrints/Classes/BPI_Interact.Set Is Targeted?`
  (params (`Is Targeted` :type Boolean))
  (set `self.Is Targeted?` `Is Targeted`))

(fn `Get Description`
  (returns (Description :type String))
  (return (`self.Description`)))

(fn `Get Name`
  (returns (Name :type String))
  (return (`self.Name`)))

(fn `Get outline Colour`
  (returns (`Outline Colour` :type "LinearColor Structure"))
  (return (`self.Outline Colour`)))

(fn `Get Outline Width`
  (returns (NewParam :type "Float (double-precision)"))
  (return (`self.Outline Width`)))

(fn `UserConstructionScript`)