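; BP_BaseLight is a base light actor that acts as a red/green indicator for an on/off state.
; Activate turns the PointLight green and Deactivate turns it red, each updating IsActive, which IsActivated reports.
; The construction script starts the light red.
; Interaction getters for name, description, type and outline return fixed values, with empty text and a zero-width outline.
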(event `/Game/BluePrints/Classes/BPI_Activation.Activate`
  (`LightComponent.SetLightColor` (`self.PointLight`) (struct :`R` 0.1247 :`G` 1.0 :`A` 1.0) true)
  (set `self.Is Active?` true))

(event `/Game/BluePrints/Classes/BPI_Activation.Deactivate`
  (`LightComponent.SetLightColor` (`self.PointLight`) (struct :`R` 1.0 :`B` 0.017423 :`A` 1.0) true)
  (set `self.Is Active?` false))

(fn `Get Description`
  (returns (Description :type String))
  (return ""))

(fn `Get Interact Type`
  (returns (NewParam :type "/Game/BluePrints/Classes/Enums/E_InteractType Enum"))
  (return "NewEnumerator4"))

(fn `Get Name`
  (returns (Name :type String))
  (return ""))

(fn `Get outline Colour`
  (returns (`Outline Colour` :type "LinearColor Structure"))
  (return))

(fn `Get Outline Width`
  (returns (NewParam :type "Float (double-precision)"))
  (return 0.0))

(fn `Is Activated?`
  (returns (`Is Activated?` :type Boolean))
  (return (`self.Is Active?`)))

(fn `UserConstructionScript`
  (`LightComponent.SetLightColor` (`self.PointLight`) (struct :`R` 1.0 :`G` 0.046328 :`B` 0.049192 :`A` 1.0) true))