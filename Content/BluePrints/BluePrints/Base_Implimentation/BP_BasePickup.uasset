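; Base pickup actor for physics objects that can be picked up, rotated while held and put down.
; Pickup turns off physics and attaches Object to a given point, keeping world rotation, while PutDown detaches and re-enables physics.
; Rotate turns the passed Direction component, caches Object's resulting world rotation, then resets Direction and reapplies that rotation to Object.
; IsRotating and SetRotationToggle are stubs returning false.
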(event `/Game/BluePrints/Classes/BPI_Pickup2.Put Down`
  (`self.K2_DetachFromActor` self "KeepWorld" "KeepWorld" "KeepWorld")
  (`PrimitiveComponent.SetSimulatePhysics` (`self.Object`) true))

(event `/Game/BluePrints/Classes/BPI_Pickup2.Rotate`
  (params (direction :type "SceneComponent Object Reference") (rotation :type "Rotator Structure"))
  (`SceneComponent.K2_AddLocalRotation` direction rotation false false)
  (set `self.Object Rotation` (`SceneComponent.K2_GetComponentRotation` (`self.Object`)))
  (`SceneComponent.K2_SetRelativeRotation` :`self` direction)
  (`SceneComponent.K2_SetWorldRotation` (`self.Object`) (`self.Object Rotation`) false false))

(fn `Get Object Rotation`
  (returns (NewParam :type "Rotator Structure"))
  (bind _output_get (set `self.Object Rotation` (`SceneComponent.K2_GetComponentRotation` (`self.Object`))))
  (return _output_get))

(fn `Is Rotating?`
  (returns (`Is Rotating?` :type Boolean))
  (return false))

(fn `Pickup`
  (params (`Attach Point` :type "SceneComponent Object Reference"))
  (returns (Actor :type "Actor Object Reference"))
  (bind _object (`self.Object`))
  (`/Engine/EditorBlueprintResources/StandardMacros.IsValid` _object
    (:`Is Valid`
      (`PrimitiveComponent.SetSimulatePhysics` _object false)
      (bind _returnvalue (`SceneComponent.K2_AttachToComponent` (`self.Object`) `Attach Point` "None" "SnapToTarget" "KeepWorld" "KeepWorld" true))
      (if _returnvalue
        (return self)
        (else
          (return null))))))

(fn `Set Rotation Toggle`
  (returns (NewParam :type Boolean))
  (return false))

(fn `UserConstructionScript`
  (`parent.UserConstructionScript`))