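; BP_BaseButton is a base pressure-button Blueprint that switches a linked ActivationTarget on and off.
; Its WeightCollider responds to the first player character or any actor implementing BPI_Weight.
; On begin overlap it sends ActivateMessage if the target reports it is not already active.
; On end overlap it sends DeactivateMessage for any qualifying actor, without checking for others still on the button.
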(event `self.ReceiveTick`
  (params (DeltaSeconds :type "Float (single-precision)"))
  (`parent.ReceiveTick` DeltaSeconds))

(event `self.Weight Collider.OnComponentBeginOverlap`
  (params (OverlappedComponent :type "PrimitiveComponent Object Reference") (OtherActor :type "Actor Object Reference") (OtherComp :type "PrimitiveComponent Object Reference") (OtherBodyIndex :type Integer) (bFromSweep :type Boolean) (SweepResult :type "HitResult Structure (by ref)"))
  (bind _activation_target (`self.Activation Target`)
    (:`then`
      (bind _is_activated_ (message `/Game/BluePrints/Classes/BPI_Activation.Is Activated?` _activation_target))
      (if (and (not _is_activated_) (or (`KismetSystemLibrary.DoesImplementInterface` OtherActor "/Game/BluePrints/Classes/BPI_Weight.BPI_Weight_C") (== OtherActor (`GameplayStatics.GetPlayerCharacter` 0))))
        (bind _activation_target_2 (`self.Activation Target`)
          (:`then`
            (message `/Game/BluePrints/Classes/BPI_Activation.Activate` _activation_target_2))
          (:`else`))))
    (:`else`)))

(event `self.Weight Collider.OnComponentEndOverlap`
  (params (OverlappedComponent :type "PrimitiveComponent Object Reference") (OtherActor :type "Actor Object Reference") (OtherComp :type "PrimitiveComponent Object Reference") (OtherBodyIndex :type Integer))
  (if (not (`KismetMathLibrary.BooleanNOR` (`KismetSystemLibrary.DoesImplementInterface` OtherActor "/Game/BluePrints/Classes/BPI_Weight.BPI_Weight_C") (== OtherActor (`GameplayStatics.GetPlayerCharacter` 0))))
    (bind _activation_target (`self.Activation Target`)
      (:`then`
        (message `/Game/BluePrints/Classes/BPI_Activation.Deactivate` _activation_target))
      (:`else`))))

(fn `UserConstructionScript`
  (`parent.UserConstructionScript`))