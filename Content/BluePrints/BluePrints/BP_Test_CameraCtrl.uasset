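; BP_Test_CameraCtrl is a test trigger-volume camera that takes over the player's view while they are inside its box.
; Box overlap begin and end call the player's EventCameraChange with zero blend time, switching to this actor and back, and toggle CameraChanged.
; Tick, gated on CameraChanged, aims the camera at the player's mesh and copies that rotation to the controller's control rotation.
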(event `self.ReceiveTick`
  (params (DeltaSeconds :type "Float (single-precision)"))
  (bind _camera (`self.Camera`))
  (`self.Camera Changed`
    (:`then`
      (bind _output_get (set `self.cam rotate` (`KismetMathLibrary.FindLookAtRotation` (`SceneComponent.K2_GetComponentLocation` _camera) (`SceneComponent.K2_GetComponentLocation` (`Character.Mesh` (`self.Player`))))))
      (`SceneComponent.K2_SetWorldRotation` _camera _output_get false false)
      (`Controller.SetControlRotation` (`self.player controller`) (`self.cam rotate`)))
    (:`else`)))

(event `self.ReceiveBeginPlay`
  (bind _bp_player (`/Game/Blueprints/Blueprints/BPF_Casts.Get Player Character` 0))
  (set `self.Player` _bp_player)
  (bind _returnvalue (`/Game/Blueprints/Blueprints/BPF_Casts.Get Player Controller` 0))
  (set `self.player controller` _returnvalue))

(event `self.Box.OnComponentBeginOverlap`
  (params (OverlappedComponent :type "PrimitiveComponent Object Reference") (OtherActor :type "Actor Object Reference") (OtherComp :type "PrimitiveComponent Object Reference") (OtherBodyIndex :type Integer) (bFromSweep :type Boolean) (SweepResult :type "HitResult Structure (by ref)"))
  (bind _player (`self.Player`))
  (if (== OtherActor _player)
    (`/Game/ThirdPerson/Blueprints/BP_ThirdPersonCharacter.Event Camera Change` _player self 0.0)
    (set `self.Camera Changed` true)))

(event `self.Box.OnComponentEndOverlap`
  (params (OverlappedComponent :type "PrimitiveComponent Object Reference") (OtherActor :type "Actor Object Reference") (OtherComp :type "PrimitiveComponent Object Reference") (OtherBodyIndex :type Integer))
  (bind _player (`self.Player`))
  (if (== _player OtherActor)
    (`/Game/ThirdPerson/Blueprints/BP_ThirdPersonCharacter.Event Camera Change` _player _player 0.0)
    (set `self.Camera Changed` false)))

(fn `UserConstructionScript`)