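; BP_Checkpoint is a checkpoint actor that records the player's save point when they pass through it.
; BeginPlay caches the player reference, and the SetCheckpoint component's begin-overlap event filters for that player.
; On overlap it calls EventSetSavePoint on the player with the current level name and the checkpoint's root transform, its location offset by SpawnLoc.
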(event `self.ReceiveBeginPlay`
  (bind _player (`/Game/BluePrints/Classes/BPF_Casts.Cast To player` 0))
  (set `self.Player` _player))

(event `self.Set Checkpoint.OnComponentBeginOverlap`
  (params (OverlappedComponent :type "PrimitiveComponent Object Reference") (OtherActor :type "Actor Object Reference") (OtherComp :type "PrimitiveComponent Object Reference") (OtherBodyIndex :type Integer) (bFromSweep :type Boolean) (SweepResult :type "HitResult Structure (by ref)"))
  (bind (_returnvalue_location _returnvalue_rotation _returnvalue_scale) (`KismetMathLibrary.BreakTransform` (`SceneComponent.K2_GetComponentToWorld` (`self.DefaultSceneRoot`))))
  (if (== OtherActor (`self.Player`))
    (bind _returnvalue (`GameplayStatics.GetCurrentLevelName` true))
    (`/Game/FirstPerson/Blueprints/BP_FirstPersonCharacter.Event Set Save point ` (`self.Player`) (`KismetMathLibrary.MakeTransform` (+ (`self.Spawn Loc`) _returnvalue_location) _returnvalue_rotation _returnvalue_scale) _returnvalue)))

(fn `UserConstructionScript`)