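; BP_Pickup is a pickup Blueprint that exposes its name, description, object type and rotation through getter functions.
; Name and description come from stored variables, and the type is a fixed enum value.
; GetObjectRotation passes the Box component's world rotation through FixAllAngles, caches the result in ObjectRotation and returns it.
; The event graph and construction script contain no logic.
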(event `GetObjectRotation_1_1`)

(fn `GetDescription`
  (returns (Description :type String))
  (return (`self.Description_0`)))

(fn `GetName`
  (returns (Name :type String))
  (return (`self.Name_0`)))

(fn `GetObjectRotation`
  (returns (`Object rotation` :type "Rotator Structure"))
  (bind _out_rotate (`/Game/BluePrints/Classes/BPF_Translation.Fix All Angles` (`SceneComponent.K2_GetComponentRotation` (`self.Box`))))
  (bind _output_get (set `self.Object Rotation` _out_rotate))
  (return _output_get))

(fn `GetObjectType`
  (returns (NewParam :type "/Game/BluePrints/Classes/Enums/E_PickupType Enum"))
  (return "NewEnumerator0"))

(fn `UserConstructionScript`)