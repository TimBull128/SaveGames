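; BP_TestPlayer_Teleport_End appears to be the exit end of a test teleport portal, positioning its PortalCam relative to its Frame.
; Each tick, while ShouldRotate is valid, it applies the rotation, scale and location offset from PortalCamRotation to the camera.
; The camera's X stays just offset from the frame, Y is clamped to corner-based bounds, and Z between world zero and the upper bound.
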(event `self.ReceiveTick`
  (params (DeltaSeconds :type "Float (single-precision)"))
  (bind _portal_cam_rotation (`self.Portal Cam Rotation`))
  (bind (_relative_upper_lef_x _relative_upper_lef_y) (`KismetMathLibrary.BreakVector` (`self.Relative Upper Lef`)))
  (bind (_relative_upper_right_x _relative_upper_right_y _relative_upper_right_z) (`KismetMathLibrary.BreakVector` (`self.Relative Upper Right`)))
  (bind (_returnvalue_x _returnvalue_y _returnvalue_z) (`KismetMathLibrary.BreakVector` (`SceneComponent.K2_GetComponentLocation` (`self.Frame`))))
  (bind (_returnvalue_x_2 _returnvalue_y_2 _returnvalue_z_2) (`KismetMathLibrary.BreakVector` (`SceneComponent.K2_GetComponentLocation` (`self.Frame`))))
  (`self.Should Rotate`
    (:`then`
      (`SceneComponent.K2_SetWorldTransform` (`self.Portal_cam`) (`KismetMathLibrary.MakeTransform` (`KismetMathLibrary.MakeVector` (- _returnvalue_x_2 15.0) (`KismetMathLibrary.FClamp` (+ _returnvalue_y_2 (.y (.location _portal_cam_rotation))) (- _returnvalue_y_2 _relative_upper_lef_y) (+ _relative_upper_right_y _returnvalue_y)) (`KismetMathLibrary.FClamp` (+ _returnvalue_z_2 (.z (.location _portal_cam_rotation))) 0.0 (+ _relative_upper_right_z _returnvalue_z))) (.rotation _portal_cam_rotation) (.scale _portal_cam_rotation)) false false))
    (:`else`)))

(fn `UserConstructionScript`)