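; BP_Door is an interactable door that, unless locked, swings its mesh through 90 degrees on a Timeline when InteractDoor fires.
; A Timeline event track sets DoorOpen by direction and plays an attenuated open or latch sound.
; With AutoClose on, Tick reverses the Timeline after a fixed or random delay while the player is within Distance.
; The construction script poses the door from DoorOpen.
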(event `self.ReceiveBeginPlay`
  ; Get Character Ref
  (bind _player_ref (`/Game/Blueprints/BFL_PlayerCast.Get Player Ref` 0))
  (set `self.PlayerRef` _player_ref))

(event `Interact Door`
  ; Checking if the door is locked
  (if (not (`self.Door locked`))
    ; Handle Animations
    (bind (_direction _lerp) (`Timeline|Timeline` :!label _label)
      (:`Update`
        (`SceneComponent.K2_SetRelativeRotation` (`self.SM_Door`) (`KismetMathLibrary.MakeRotator` 0.0 0.0 (* _lerp 90.0)) false false))
      (:`Door_opening`
        ; play sound on open and close door
        (switch `ETimelineDirection` _direction
          (:`Forward`
            (bind _output_get (set `self.Door Open` true)))
          (:`Backward`
            (set `self.Door Open` false)))
        (`GameplayStatics.PlaySoundAtLocation` (select `int` (`KismetMathLibrary.SelectInt` 0 1 _output_get) :`0` "/Game/Blueprints/sounds/door-opening.door-opening" :`1` "/Game/Blueprints/sounds/door_latch.door_latch" :!type "SoundBase Object Reference") (0.0 0.0 0.0) (struct) 0.5 1.0 0.0 "/Game/Blueprints/sounds/SAT_door.SAT_door" null self null)))))

(event `self.ReceiveTick`
  (params (DeltaSeconds :type "Float (single-precision)"))
  ; Automatically Close door
  (bind (_delay _close_door) (`self.Auto Close Delay` (`self.PlayerRef`)))
  (if (and _close_door (`self.Door Open`))
    (`KismetSystemLibrary.Delay` _delay)
    (goto _label :!via `Reverse`)))

(fn `Auto Close Delay`
  (params (Actor :type "Actor Object Reference (by ref)"))
  (returns (Delay :type "Float (double-precision)") (`Close Door` :type Boolean))
  (locals (`Curr Delay` :type "Float (double-precision)" :default 0.0))
  (bind _close_delay (`self.Close Delay`))
  (return (`KismetMathLibrary.SelectFloat` (`KismetMathLibrary.RandomFloatInRange` 0.0 _close_delay) _close_delay (`self.Random Delay`)) (and (< (`self.GetDistanceTo` Actor) (`self.Distance`)) (`self.Auto Close`))))

(fn `UserConstructionScript`
  (`SceneComponent.K2_SetRelativeRotation` (`self.SM_Door`) (`KismetMathLibrary.MakeRotator` 0.0 0.0 (`KismetMathLibrary.SelectFloat` 90.0 0.0 (`self.Door Open`))) false false))