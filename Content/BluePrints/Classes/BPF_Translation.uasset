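; Blueprint function library of rotation helpers that add rotators and keep their angles within 0 to 360 degrees.
; UpdateRotator sums two rotators per axis and passes the result through FixAllAngles, which runs FixAngle on roll, pitch and yaw.
; FixAngle wraps by repeatedly adding or subtracting a full turn in while loops, leaving exactly 360 unchanged.
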(fn `Fix All Angles`
  (params (Rotator :type "Rotator Structure"))
  (returns (`Out rotate` :type "Rotator Structure"))
  (return (`KismetMathLibrary.MakeRotator` (`self.Fix Angle` Rotator_Roll) (`self.Fix Angle` Rotator_Pitch) (`self.Fix Angle` Rotator_Yaw))))

(fn `Fix Angle`
  (params (Angle :type "Float (double-precision)"))
  (returns (`Out Angle` :type "Float (double-precision)"))
  (locals (`Return Angle` :type "Float (double-precision)"))
  (bind _output_get (set `local.Return Angle` Angle))
  (bind _returnvalue (< _output_get 0.0))
  (if _returnvalue
    (while _returnvalue
      (set `local.Return Angle` (+ (`local.Return Angle`) 360.0)))
    (return (`local.Return Angle`))
    (else
      (bind _returnvalue_2 (> _output_get 360.0))
      (if _returnvalue_2
        (while _returnvalue_2
          (set `local.Return Angle` (- (`local.Return Angle`) 360.0)))
        (return (`local.Return Angle`))
        (else
          (return (`local.Return Angle`)))))))

(fn `Update Rotator`
  (params (`Initial Target` :type "Rotator Structure") (`Add Rotator` :type "Rotator Structure"))
  (returns (`Result Rotator` :type "Rotator Structure"))
  (bind _out_rotate (`self.Fix All Angles` (`KismetMathLibrary.MakeRotator` (+ `Initial Target_Roll` `Add Rotator_Roll`) (+ `Initial Target_Pitch` `Add Rotator_Pitch`) (+ `Initial Target_Yaw` `Add Rotator_Yaw`))))
  (return _out_rotate))