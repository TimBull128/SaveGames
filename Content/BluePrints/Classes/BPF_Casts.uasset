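; Blueprint function library of shared helpers for managing BP_Save save games and fetching the first-person player character.
; GetSaveState loads an existing slot or creates a new save stamped with slot name and user index, flagging whether it is new.
; SaveGameState writes to the slot stored on the save object itself, while DeleteSaveState clears a given slot.
; CastToPlayer returns the character at a player index as BP_FirstPersonCharacter.
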(fn `Cast To player`
  (params (PlayerIndex :type Integer))
  (returns (Player :type "/Game/FirstPerson/Blueprints/BP_FirstPersonCharacter Object Reference"))
  (bind _asbp_first_person_character (cast `/Game/FirstPerson/Blueprints/BP_FirstPersonCharacter` (`GameplayStatics.GetPlayerCharacter` null PlayerIndex)))
  (return _asbp_first_person_character))

(fn `Create Save state`
  (returns (ReturnValue :type "/Game/BluePrints/Classes/BP_Save Object Reference"))
  (bind _returnvalue (`GameplayStatics.CreateSaveGameObject` "/Game/BluePrints/Classes/BP_Save.BP_Save_C"))
  (return _returnvalue))

(fn `Delete Save State`
  (params (SlotName :type String) (UserIndex :type Integer))
  (returns (ReturnValue :type Boolean))
  (bind _returnvalue (`GameplayStatics.DeleteGameInSlot` SlotName UserIndex))
  (return _returnvalue))

(fn `Get Save State`
  (params (`Slot Name` :type String) (`User Index` :type Integer))
  (returns (`Save Output` :type "/Game/BluePrints/Classes/BP_Save Object Reference") (`New State?` :type Boolean))
  (locals (`Slot Name Ref` :type String) (`User Index Ref` :type Integer) (`Player Transform Ref` :type "Transform Structure"))
  (set `local.Slot Name Ref` `Slot Name`)
  (set `local.User Index Ref` `User Index`)
  (bind _returnvalue (`GameplayStatics.DoesSaveGameExist` (`local.Slot Name Ref`) (`local.User Index Ref`)))
  (if _returnvalue
    (bind _save_output (`self.Load Save State` null (`local.Slot Name Ref`) (`local.User Index Ref`)))
    (return _save_output false)
    (else
      (bind _returnvalue_2 (`self.Create Save state` null))
      (set `/Game/BluePrints/Classes/BP_Save.User Slot` (`local.User Index Ref`) _returnvalue_2)
      (set `/Game/BluePrints/Classes/BP_Save.Save Name` (`local.Slot Name Ref`) _returnvalue_2)
      (return _returnvalue_2 true))))

(fn `Load Save State`
  (params (SlotName :type String) (UserIndex :type Integer))
  (returns (`Save Output` :type "/Game/BluePrints/Classes/BP_Save Object Reference"))
  (bind _returnvalue (`GameplayStatics.LoadGameFromSlot` SlotName UserIndex))
  (bind _asbp_save (cast `/Game/BluePrints/Classes/BP_Save` _returnvalue))
  (return _asbp_save))

(fn `Save Game State`
  (params (`Save Game` :type "/Game/BluePrints/Classes/BP_Save Object Reference"))
  (returns (`Complete?` :type Boolean))
  (bind _returnvalue (`GameplayStatics.SaveGameToSlot` `Save Game` (`/Game/BluePrints/Classes/BP_Save.Save Name` `Save Game`) (`/Game/BluePrints/Classes/BP_Save.User Slot` `Save Game`)))
  (return _returnvalue))